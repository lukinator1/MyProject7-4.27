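; Blind spell that the Protagonist casts to temporarily take away an Enemy1's sight.
; Cast runs a camera-forward line trace, flags the enemy hit as Blinded, disables its AI sight sense, clears its perception memory and attaches a Niagara effect to its mesh.
; A timer then calls Remove Blind to destroy the effect and restore sight.
; If the trace finds no Enemy1, it clears the spell timer and ends the cooldown.
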(event `self.Cast`
  (bind _asprotagonist (cast `/Game/Blueprints/Protagonist` (`self.GetInstigator`)))
  (bind _firstpersoncamera (`/Game/Blueprints/Protagonist.firstpersoncamera` _asprotagonist))
  (bind _returnvalue (`SceneComponent.K2_GetComponentLocation` _firstpersoncamera))
  (bind _returnvalue_2 (`SceneComponent.K2_GetComponentRotation` _firstpersoncamera))
  (bind _outhit (`KismetSystemLibrary.LineTraceSingle` :`Start` (+ _returnvalue (`KismetMathLibrary.GreaterGreater_VectorRotator` (40.0 0.0 0.0) _returnvalue_2)) :`End` (+ _returnvalue (`KismetMathLibrary.GreaterGreater_VectorRotator` (1500.0 0.0 0.0) _returnvalue_2)) :`TraceChannel` "TraceTypeQuery2" :`DrawTime` 2.5))
  (bind _asenemy_1 (cast `/Game/Blueprints/Enemy1` (`.HitActor` (`GameplayStatics.BreakHitResult` _outhit)))
    (:`then`
      (set `/Game/Blueprints/Enemy1.Blinded` true _asenemy_1)
      (bind _returnvalue_3 (`AIController.GetAIPerceptionComponent` (`AIBlueprintHelperLibrary.GetAIController` _asenemy_1)))
      (`AIPerceptionComponent.SetSenseEnabled` _returnvalue_3 "/Script/AIModule.AISense_Sight" false)
      (`AIPerceptionComponent.ForgetAll` _returnvalue_3)
      (bind _returnvalue_4 (`AddComponent|NODE_AddNiagaraComponent-0` :`self` _asenemy_1 :`RelativeTransform` (`KismetMathLibrary.MakeTransform` (15.0 -21.0 0.0))))
      (`SceneComponent.K2_AttachToComponent` _returnvalue_4 (`Character.Mesh` _asenemy_1) "Hat" "KeepRelative" "KeepRelative" "KeepRelative" true)
      (`NiagaraComponent.SetAsset` _returnvalue_4 "/Game/Blueprints/InvisiblityNiagara.InvisiblityNiagara" true)
      (set `self.Blind Niagaracomponent` _returnvalue_4)
      (set `self.Blinded Enemy` _asenemy_1)
      (`KismetSystemLibrary.K2_SetTimer` null "Remove Blind" 8.0))
    (:`CastFailed`
      (`KismetSystemLibrary.K2_ClearAndInvalidateTimerHandle` (`self.spelltimerhandle`))
      (`self.endCooldown`))))

(fn `Remove Blind`
  (bind _blinded_enemy (`self.Blinded Enemy`))
  (if (!= _blinded_enemy null)
    (`ActorComponent.K2_DestroyComponent` (`self.Blind Niagaracomponent`) _blinded_enemy)
    (`AIPerceptionComponent.SetSenseEnabled` (`AIController.GetAIPerceptionComponent` (`AIBlueprintHelperLibrary.GetAIController` _blinded_enemy)) "/Script/AIModule.AISense_Sight" true)
    (set `/Game/Blueprints/Enemy1.Blinded` false _blinded_enemy)))

(fn `UserConstructionScript`)