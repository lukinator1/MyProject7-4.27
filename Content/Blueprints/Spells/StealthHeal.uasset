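; StealthHeal is a spell Blueprint that heals the casting Protagonist, favouring casts made while undetected.
; On Cast, it reads the Alert flag from MyGameStateBase and calls Heal on the Protagonist instigator, with a larger amount when the alert is off.
; All logic sits in the Cast event; BeginPlay, overlap, Tick and the construction script are empty.
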(event `self.Cast`
  (if true
    (bind _asmy_game_state_base (cast `/Game/Blueprints/MyGameStateBase` (`GameplayStatics.GetGameState`)))
    (if (`/Game/Blueprints/MyGameStateBase.Alert` _asmy_game_state_base)
      (bind _asprotagonist (cast `/Game/Blueprints/Protagonist` (`self.GetInstigator`)))
      (`/Game/Blueprints/Protagonist.Heal` _asprotagonist 20.0 null)
      (else
        (bind _asprotagonist_2 (cast `/Game/Blueprints/Protagonist` (`self.GetInstigator`)))
        (`/Game/Blueprints/Protagonist.Heal` _asprotagonist_2 50.0 null)))))

(fn `UserConstructionScript`)