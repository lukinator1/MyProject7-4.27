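; MoveEnemy is a two-cast spell that lets the Protagonist pick an enemy and teleport it elsewhere.
; Each cast line-traces from the first-person camera; with nothing selected, a hit Enemy gets a highlight material and is stored, and the cooldown ends immediately either way.
; With an enemy selected, the cast restores its material, teleports it to the hit point or trace end, and clears the selection, leaving the cooldown intact.
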(event `self.Cast`
  (bind _selected (`self.Selected`))
  (bind _returnvalue (`self.K2_GetActorRotation` _selected))
  (bind _asprotagonist (cast `/Game/Blueprints/Protagonist` (`self.GetInstigator`)))
  (bind _firstpersoncamera (`/Game/Blueprints/Protagonist.firstpersoncamera` _asprotagonist))
  (bind _returnvalue_2 (`SceneComponent.K2_GetComponentLocation` _firstpersoncamera))
  (bind _returnvalue_3 (`SceneComponent.K2_GetComponentRotation` _firstpersoncamera))
  (bind (_outhit _returnvalue_4) (`KismetSystemLibrary.LineTraceSingle` :`Start` (+ _returnvalue_2 (`KismetMathLibrary.GreaterGreater_VectorRotator` (40.0 0.0 0.0) _returnvalue_3)) :`End` (+ _returnvalue_2 (`KismetMathLibrary.GreaterGreater_VectorRotator` (2200.0 0.0 0.0) _returnvalue_3)) :`TraceChannel` "TraceTypeQuery2" :`DrawTime` 2.5))
  (if (!= _selected null)
    (`PrimitiveComponent.SetMaterial` (`Character.Mesh` (`self.Selected`)) 0 (`Enemy.baseenemymaterial` _selected))
    (if _returnvalue_4
      (bind (_bblockinghit _binitialoverlap _time _distance _location _impactpoint _normal _impactnormal _physmat _hitactor _hitcomponent _hitbonename _hititem _elementindex _faceindex _tracestart _traceend) (`GameplayStatics.BreakHitResult` _outhit))
      (`self.K2_TeleportTo` _selected _location _returnvalue)
      (else
        (`self.K2_TeleportTo` _selected _traceend _returnvalue)))
    (set `self.Selected` null)
    (else
      (bind _asenemy (cast `Enemy` _hitactor)
        (:`then`
          (`PrimitiveComponent.SetMaterial` (`Character.Mesh` _asenemy) 0 "/Game/TeleportEnemyMaterial.TeleportEnemyMaterial")
          (set `self.Selected` _asenemy))
        (:`CastFailed`
          _))
      (`KismetSystemLibrary.K2_ClearAndInvalidateTimerHandle` (`self.spelltimerhandle`))
      (`self.endCooldown`))))

(fn `UserConstructionScript`)