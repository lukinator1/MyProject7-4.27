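; Invisibility spell actor that toggles invisibility on the Protagonist who instigates it.
; Casting flags the player invisible, hides the actor in game and unregisters its AI perception stimuli source from sight.
; A short timer then calls Cancel invisibility to restore visibility and sight registration; casting again while invisible clears the timer and cancels immediately.
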(event `self.Cast`
  (bind _returnvalue (`self.GetInstigator`))
  (bind _asprotagonist (cast `/Game/Blueprints/Protagonist` _returnvalue))
  (if (`/Game/Blueprints/Protagonist.Invisible` _asprotagonist)
    (set `/Game/Blueprints/Protagonist.Invisible` false _asprotagonist)
    (`KismetSystemLibrary.K2_ClearAndInvalidateTimerHandle` (`self.Cancel invisiblity handle`))
    (`self.Cancel invisibility`)
    (else
      (set `/Game/Blueprints/Protagonist.Invisible` true _asprotagonist)
      (`AIPerceptionStimuliSourceComponent.UnregisterFromSense` (`/Game/Blueprints/Protagonist.AIPerceptionStimuliSource` _asprotagonist) "/Script/AIModule.AISense_Sight")
      (`self.SetActorHiddenInGame` _returnvalue true)
      (bind _returnvalue_2 (`KismetSystemLibrary.K2_SetTimer` null "Cancel invisibility" 2.5))
      (set `self.Cancel invisiblity handle` _returnvalue_2))))

(fn `Cancel invisibility`
  (bind _returnvalue (`self.GetInstigator`))
  (bind _asprotagonist (cast `/Game/Blueprints/Protagonist` _returnvalue))
  (set `/Game/Blueprints/Protagonist.Invisible` false _asprotagonist)
  (`AIPerceptionStimuliSourceComponent.RegisterForSense` (`/Game/Blueprints/Protagonist.AIPerceptionStimuliSource` _asprotagonist) "/Script/AIModule.AISense_Sight")
  (`self.SetActorHiddenInGame` _returnvalue false))

(fn `UserConstructionScript`)