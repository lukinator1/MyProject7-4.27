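; Smoke screen spell that places a SmokeScreenCloud actor where the casting Protagonist is aiming.
; On Cast, it line traces on the Camera channel forward from the instigator's first-person camera, starting just ahead of it.
; The cloud spawns at the hit point, or at the trace's end when nothing is hit, and the spell stores a reference to it.
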(event `self.Cast`
  (bind _asprotagonist (cast `/Game/Blueprints/Protagonist` (`self.GetInstigator`)))
  (bind _firstpersoncamera (`/Game/Blueprints/Protagonist.firstpersoncamera` _asprotagonist))
  (bind _returnvalue (`SceneComponent.K2_GetComponentLocation` _firstpersoncamera))
  (bind _returnvalue_2 (`SceneComponent.K2_GetComponentRotation` _firstpersoncamera))
  (bind (_outhit _returnvalue_3) (`KismetSystemLibrary.LineTraceSingle` :`Start` (+ _returnvalue (`KismetMathLibrary.GreaterGreater_VectorRotator` (40.0 0.0 0.0) _returnvalue_2)) :`End` (+ _returnvalue (`KismetMathLibrary.GreaterGreater_VectorRotator` (2200.0 0.0 0.0) _returnvalue_2)) :`TraceChannel` "TraceTypeQuery2" :`DrawTime` 2.5))
  (if _returnvalue_3
    (bind (_bblockinghit _binitialoverlap _time _distance _location _impactpoint _normal _impactnormal _physmat _hitactor _hitcomponent _hitbonename _hititem _elementindex _faceindex _tracestart _traceend) (`GameplayStatics.BreakHitResult` _outhit))
    (bind _returnvalue_4 (`|SpawnActorFromClass` "/Game/Blueprints/Smokescreencloud.SmokeScreenCloud_C" (`KismetMathLibrary.Conv_VectorToTransform` _location) "Undefined" "OverrideRootScale" null null))
    (set `self.Smokescreen cloud` _returnvalue_4)
    (else
      (bind _returnvalue_5 (`|SpawnActorFromClass` "/Game/Blueprints/Smokescreencloud.SmokeScreenCloud_C" (`KismetMathLibrary.Conv_VectorToTransform` _traceend) "Undefined" "OverrideRootScale" null null))
      (set `self.Smokescreen cloud` _returnvalue_5))))

(fn `UserConstructionScript`)