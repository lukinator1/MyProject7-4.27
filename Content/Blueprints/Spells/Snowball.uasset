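; Snowball spell that, when cast, launches a small SnowBall_Ball actor from the Protagonist's first-person view.
; Cast gets the Protagonist from the Instigator, spawns the ball slightly ahead of the camera with a yaw-offset camera rotation, and passes the Instigator along.
; Stun-removal logic (repossessing the enemy, restoring its material) is disconnected in both graphs, leaving CancelStun empty.
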(event `self.Cast`
  (bind _asprotagonist (cast `/Game/Blueprints/Protagonist` (`self.Instigator`)))
  (bind _rotation (.rotation (`SceneComponent.K2_GetComponentToWorld` (`/Game/Blueprints/Protagonist.firstpersoncamera` _asprotagonist))))
  (`|SpawnActorFromClass` "/Game/Blueprints/SnowBall_Ball.SnowBall_Ball_C" (`KismetMathLibrary.MakeTransform` (+ (.location (`SceneComponent.K2_GetComponentToWorld` (`/Game/Blueprints/Protagonist.firstpersoncamera` _asprotagonist))) (`KismetMathLibrary.GreaterGreater_VectorRotator` (40.0 0.0 0.0) _rotation)) (`KismetMathLibrary.ComposeRotators` (struct :`Pitch` 90.0) _rotation) (0.15 0.15 0.15)) "Undefined" "OverrideRootScale" null (`self.GetInstigator`)))

(fn `Cancel stun`)

(fn `UserConstructionScript`)