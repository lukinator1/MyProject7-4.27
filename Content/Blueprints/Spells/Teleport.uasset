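; Teleport spell that moves the instigating Protagonist to where they are looking when cast.
; A camera-channel line trace runs forward from the first-person camera; on a miss, the player teleports to the trace end.
; On a hit, it teleports to the impact point, and if that fails, retries in growing steps along the surface normal until it succeeds or reaches a limit.
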(event `self.Cast`
  (bind _i (`self.i`))
  (bind _asprotagonist (cast `/Game/Blueprints/Protagonist` (`self.GetInstigator`)))
  (bind _firstpersoncamera (`/Game/Blueprints/Protagonist.firstpersoncamera` _asprotagonist))
  (bind _returnvalue (`SceneComponent.K2_GetComponentLocation` _firstpersoncamera))
  (bind _returnvalue_2 (`SceneComponent.K2_GetComponentRotation` _firstpersoncamera))
  (bind (_outhit _returnvalue_3) (`KismetSystemLibrary.LineTraceSingle` :`Start` (+ _returnvalue (`KismetMathLibrary.GreaterGreater_VectorRotator` (110.0 0.0 0.0) _returnvalue_2)) :`End` (+ _returnvalue (`KismetMathLibrary.GreaterGreater_VectorRotator` (3000.0 0.0 0.0) _returnvalue_2)) :`TraceChannel` "TraceTypeQuery2" :`DrawTime` 2.5))
  (if _returnvalue_3
    ;[1 1 1] Brute force method of attempting to resolve collisions should Unreal's teleport fail
    (set `self.i` 0)
    (bind (_bblockinghit _binitialoverlap _time _distance _location _impactpoint _normal _impactnormal _physmat _hitactor _hitcomponent _hitbonename _hititem _elementindex _faceindex _tracestart _traceend) (`GameplayStatics.BreakHitResult` _outhit))
    (set `self.targetlocation` _location)
    (bind _returnvalue_4 (`self.K2_GetActorRotation` _asprotagonist))
    (bind _returnvalue_5 (`self.K2_TeleportTo` _asprotagonist (`self.targetlocation`) _returnvalue_4 :!label _label))
    (if (and (not _returnvalue_5) (<= _i 120))
      (bind _output_get (set `self.i` (+ 10 _i)))
      (set `self.targetlocation` (+ _location (* _normal _i)))
      (goto _label))
    (else
      (`self.K2_TeleportTo` _asprotagonist _traceend _returnvalue_4))))

(fn `NewFunction_0`)

(fn `NewFunction_1`)

(fn `NewFunction_2`)

(fn `UserConstructionScript`)