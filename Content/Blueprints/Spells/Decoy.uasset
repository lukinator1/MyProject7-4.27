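; Decoy spell that spawns a temporary AI copy of the Protagonist where the casting player is looking.
; On Cast, a short line trace from the first-person camera picks the spawn point, using the hit location or the trace end.
; After spawning, the player controller re-possesses the original Protagonist, and a timer destroys the stored decoy after a fixed lifetime.
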(event `self.Cast`
  (bind _asprotagonist (cast `/Game/Blueprints/Protagonist` (`self.GetInstigator`)))
  (bind _firstpersoncamera (`/Game/Blueprints/Protagonist.firstpersoncamera` _asprotagonist))
  (bind _returnvalue (`SceneComponent.K2_GetComponentLocation` _firstpersoncamera))
  (bind _returnvalue_2 (`SceneComponent.K2_GetComponentRotation` _firstpersoncamera))
  (bind (_outhit _returnvalue_3) (`KismetSystemLibrary.LineTraceSingle` :`Start` (+ _returnvalue (`KismetMathLibrary.GreaterGreater_VectorRotator` (40.0 0.0 0.0) _returnvalue_2)) :`End` (+ _returnvalue (`KismetMathLibrary.GreaterGreater_VectorRotator` (600.0 0.0 0.0) _returnvalue_2)) :`TraceChannel` "TraceTypeQuery2" :`DrawTime` 6.0))
  (if _returnvalue_3
    (bind (_bblockinghit _binitialoverlap _time _distance _location _impactpoint _normal _impactnormal _physmat _hitactor _hitcomponent _hitbonename _hititem _elementindex _faceindex _tracestart _traceend) (`GameplayStatics.BreakHitResult` _outhit))
    (bind _returnvalue_4 (`AIBlueprintHelperLibrary.SpawnAIFromClass` "/Game/Blueprints/ProtagonistDecoy.ProtagonistDecoy_C" null _location (struct) false null))
    (bind _asprotagonist_2 (cast `/Game/Blueprints/Protagonist` _returnvalue_4))
    (set `self.Decoy` _asprotagonist_2)
    (else
      (bind _returnvalue_5 (`AIBlueprintHelperLibrary.SpawnAIFromClass` "/Game/Blueprints/ProtagonistDecoy.ProtagonistDecoy_C" null _traceend (struct) false null))
      (bind _asprotagonist_3 (cast `/Game/Blueprints/Protagonist` _returnvalue_5))
      (set `self.Decoy` _asprotagonist_3)))
  (`Controller.Possess` (`GameplayStatics.GetPlayerControllerFromID` 0) _asprotagonist)
  (`KismetSystemLibrary.K2_SetTimer` null "Destroy decoy" 15.0))

(fn `Destroy decoy`
  (bind _decoy (`self.Decoy`))
  (if (not (== _decoy null))
    (`self.K2_DestroyActor` _decoy)))

(fn `UserConstructionScript`)