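; Game state for a stealth game that tracks the alert state and drives the background music to match it.
; An audio component starts on BeginPlay; StartAlert and EndAlert toggle the Alert flag and swap tracks, with EndAlert leaving the rest and game over tracks untouched.
; Gameover plays its own track, then a timer runs Reset Game, which ends every alerted enemy's AI investigation and restores the rest music.
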(event `self.ReceiveBeginPlay`
  (`AudioComponent.Play` (`self.Currentsong`) 0.0))

(event `self.ReceiveTick`
  (params (DeltaSeconds :type "Float (single-precision)")))

(fn `EndAlert`
  (bind _currentsong (`self.Currentsong`))
  (bind _sound (`AudioComponent.Sound` _currentsong))
  (if (and (!= _sound "/Game/all-star-rest-area-super-smash-bros_melee-gabed_net.all-star-rest-area-super-smash-bros_melee-gabed_net") (!= _sound "/Game/Metal_Gear_Solid_Game_Over_screen__Clean_background_.Metal_Gear_Solid_Game_Over_screen__Clean_background_"))
    (`AudioComponent.SetSound` _currentsong "/Game/all-star-rest-area-super-smash-bros_melee-gabed_net.all-star-rest-area-super-smash-bros_melee-gabed_net"))
  (set `self.Alert` false))

(fn `Gameover`
  (`AudioComponent.SetSound` (`self.Currentsong`) "/Game/Metal_Gear_Solid_Game_Over_screen__Clean_background_.Metal_Gear_Solid_Game_Over_screen__Clean_background_")
  (`KismetSystemLibrary.K2_SetTimer` null "Reset Game" 13.0))

(fn `Reset Game`
  (set `self.Temparray` (`self.On Alert Enemies`))
  (for _array_element (`self.Temparray`)
    (bind _asenemy_1aicontroller (cast `/Game/Blueprints/Enemy1AIController` (`AIBlueprintHelperLibrary.GetAIController` _array_element)))
    (`KismetSystemLibrary.K2_ClearAndInvalidateTimerHandle` (`/Game/Blueprints/Enemy1AIController.end investigation timer` _asenemy_1aicontroller))
    (`/Game/Blueprints/Enemy1AIController.Endinvestigation` _asenemy_1aicontroller))
  (`AudioComponent.SetSound` (`self.Currentsong`) "/Game/all-star-rest-area-super-smash-bros_melee-gabed_net.all-star-rest-area-super-smash-bros_melee-gabed_net"))

(fn `StartAlert`
  (`AudioComponent.SetSound` (`self.Currentsong`) "/Game/2rNSjhWG0S2M_128.2rNSjhWG0S2M_128")
  (set `self.Alert` true))

(fn `UserConstructionScript`)