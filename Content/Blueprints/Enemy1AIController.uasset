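; AI controller for Enemy1 that runs a behavior tree and drives its investigate, pursue and attack blackboard states.
; Perception of the Protagonist, or a decoy when not pursuing, starts investigation; losing it starts a timer to reset.
; While investigating, Tick sets pursuit and attack flags from distance, sight, invisibility, blind and stun checks.
; Pursuing enemies register with the GameState to raise a shared alert, which ends when the last one gives up.
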(event `self.ReceiveBeginPlay`
  (`self.RunBehaviorTree` "/Game/BehaviorTree.BehaviorTree"))

(event `self.ReceiveTick`
  (params (DeltaSeconds :type "Float (single-precision)"))
  (bind _returnvalue (`AIBlueprintHelperLibrary.GetBlackboard` null))
  (bind _returnvalue_2 (`self.K2_GetPawn`))
  (if (`BlackboardComponent.GetValueAsBool` _returnvalue "Investigating")
    (bind _asenemy_1 (cast `/Game/Blueprints/Enemy1` _returnvalue_2))
    (bind _asprotagonist (cast `/Game/Blueprints/Protagonist` (`BlackboardComponent.GetValueAsObject` _returnvalue "TargetActor")))
    (bind _returnvalue_3 (`KismetMathLibrary.VSize` (- (`self.K2_GetActorLocation` _returnvalue_2) (`self.K2_GetActorLocation` _asprotagonist))))
    (bind _returnvalue_4 (and (<= _returnvalue_3 1150.0) (`KismetMathLibrary.BooleanNOR` (`/Game/Blueprints/Protagonist.Invisible` _asprotagonist) (`/Game/Blueprints/Enemy1.Blinded` _asenemy_1)) (>= (`KismetArrayLibrary.Array_Length` (`AIPerceptionComponent.GetKnownPerceivedActors` (`self.AIPerception`) "/Script/AIModule.AISense_Sight")) 1) (not (`/Game/Blueprints/Enemy1.Stunned` _asenemy_1))))
    (`BlackboardComponent.SetValueAsBool` _returnvalue "Pursueplayer" _returnvalue_4)
    (if _returnvalue_4
      (`BlackboardComponent.SetValueAsBool` _returnvalue "Inattackrange" (<= _returnvalue_3 275.0))
      (if (== (`GameplayStatics.GetObjectClass` (`BlackboardComponent.GetValueAsObject` _returnvalue "TargetActor")) "/Game/Blueprints/Protagonist.Protagonist_C")
        (bind _asmy_game_state_base (cast `/Game/Blueprints/MyGameStateBase` (`GameplayStatics.GetGameState`)))
        (bind _asenemy_1_2 (cast `/Game/Blueprints/Enemy1` _returnvalue_2))
        (`KismetArrayLibrary.Array_AddUnique` (`/Game/Blueprints/MyGameStateBase.On Alert Enemies` _asmy_game_state_base) _asenemy_1_2)
        (if (not (`/Game/Blueprints/MyGameStateBase.Alert` _asmy_game_state_base))
          (`/Game/Blueprints/MyGameStateBase.StartAlert` _asmy_game_state_base)
          (`/Game/Blueprints/Enemy1.apples` _asenemy_1_2)))
      (else
        (`BlackboardComponent.SetValueAsBool` _returnvalue "Inattackrange" false)))))

(event `self.AIPerception.OnTargetPerceptionUpdated`
  (params (Actor :type "Actor Object Reference") (Stimulus :type "AIStimulus Structure"))
  (bind (_age _expirationage _strength _stimuluslocation _receiverlocation _tag _bsuccessfullysensed) (break `AIStimulus` Stimulus))
  (bind _returnvalue (`AIBlueprintHelperLibrary.GetBlackboard` null))
  (if (== (`GameplayStatics.GetObjectClass` Actor) "/Game/Blueprints/Protagonist.Protagonist_C")
    (if _bsuccessfullysensed :!label _label
      (`BlackboardComponent.SetValueAsBool` _returnvalue "Investigating" _bsuccessfullysensed)
      (`KismetSystemLibrary.K2_ClearAndInvalidateTimerHandle` (`self.end investigation timer`))
      (`BlackboardComponent.SetValueAsVector` _returnvalue "Targetplayerlocation" _stimuluslocation)
      (`BlackboardComponent.SetValueAsVector` _returnvalue "Playerlocation" _stimuluslocation)
      (`BlackboardComponent.SetValueAsObject` _returnvalue "TargetActor" Actor)
      (else
        (bind _returnvalue_2 (`KismetSystemLibrary.K2_SetTimer` null "Endinvestigation" _expirationage))
        (set `self.end investigation timer` _returnvalue_2)))
    (elif (not (or (and (== (`GameplayStatics.GetObjectClass` (`BlackboardComponent.GetValueAsObject` _returnvalue "TargetActor")) "/Game/Blueprints/Protagonist.Protagonist_C") (`BlackboardComponent.GetValueAsBool` _returnvalue "Pursueplayer")) (not (== (`GameplayStatics.GetObjectClass` Actor) "/Game/Blueprints/ProtagonistDecoy.ProtagonistDecoy_C"))))
      (goto _label))))

(event `self.AIPerception.OnTargetPerceptionInfoUpdated`
  (params (UpdateInfo :type "ActorPerceptionUpdateInfo Structure (by ref)")))

(event `self.AIPerception.OnPerceptionUpdated`
  (params (UpdatedActors :type "Array of Actor Object Reference (by ref)")))

(fn `Endinvestigation`
  (bind _returnvalue (`AIBlueprintHelperLibrary.GetBlackboard` null))
  (bind _asenemy_1 (cast `/Game/Blueprints/Enemy1` (`self.K2_GetPawn`)))
  (set `CharacterMovementComponent.MaxWalkSpeed` 600.0 (`Character.CharacterMovement` _asenemy_1))
  (`BlackboardComponent.SetValueAsBool` _returnvalue "Reachedmeanderdestination" false)
  (`BlackboardComponent.SetValueAsBool` _returnvalue "ReachedTargetPlayerLocation" false)
  (`BlackboardComponent.SetValueAsBool` _returnvalue "Investigating" false)
  (`BlackboardComponent.SetValueAsObject` _returnvalue "TargetPlayer" null)
  (bind _asmy_game_state_base (cast `/Game/Blueprints/MyGameStateBase` (`GameplayStatics.GetGameState`)))
  (bind _asenemy_1_2 (cast `/Game/Blueprints/Enemy1` (`self.K2_GetPawn`)))
  (bind _on_alert_enemies (`/Game/Blueprints/MyGameStateBase.On Alert Enemies` _asmy_game_state_base))
  (`KismetArrayLibrary.Array_RemoveItem` _on_alert_enemies _asenemy_1_2)
  (if (and (== (`KismetArrayLibrary.Array_Length` _on_alert_enemies) 0) (`/Game/Blueprints/MyGameStateBase.Alert` _asmy_game_state_base))
    (`/Game/Blueprints/MyGameStateBase.EndAlert` _asmy_game_state_base)))

(fn `UserConstructionScript`)