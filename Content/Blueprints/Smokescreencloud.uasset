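; Smoke screen cloud actor that blocks AI sight for enemies and hides the protagonist, then destroys itself after a fixed delay.
; Overlapping Enemy1 actors lose sight sense and forget perceived targets; investigating ones get a timer to end investigation.
; The protagonist unregisters as a sight stimulus and is flagged Invisible.
; Sphere end overlap reverses both effects for root components only; an initial-overlap sweep is left unconnected.
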(event `CustomEvent_1`
  (params (OtherActor :type "Actor Object Reference")))

(event `self.ReceiveActorBeginOverlap`
  (params (OtherActor :type "Actor Object Reference"))
  (bind _asenemy_1 (cast `/Game/Blueprints/Enemy1` OtherActor)
    (:`then`
      (bind _returnvalue (`AIBlueprintHelperLibrary.GetAIController` _asenemy_1))
      (bind _returnvalue_2 (`AIController.GetAIPerceptionComponent` _returnvalue))
      (`AIPerceptionComponent.SetSenseEnabled` _returnvalue_2 "/Script/AIModule.AISense_Sight" false)
      (`AIPerceptionComponent.ForgetAll` _returnvalue_2)
      (if (`BlackboardComponent.GetValueAsBool` (`AIBlueprintHelperLibrary.GetBlackboard` _returnvalue) "Investigating")
        (bind _asenemy_1aicontroller (cast `/Game/Blueprints/Enemy1AIController` _returnvalue))
        (`KismetSystemLibrary.K2_SetTimer` _asenemy_1aicontroller "Endinvestigation" 15.0)))
    (:`CastFailed`
      (bind _asprotagonist (cast `/Game/Blueprints/Protagonist` OtherActor))
      (`AIPerceptionStimuliSourceComponent.UnregisterFromSense` (`/Game/Blueprints/Protagonist.AIPerceptionStimuliSource` _asprotagonist) "/Script/AIModule.AISense_Sight")
      (set `/Game/Blueprints/Protagonist.Invisible` true _asprotagonist))))

(event `self.ReceiveTick`
  (params (DeltaSeconds :type "Float (single-precision)")))

(event `self.ReceiveBeginPlay`
  (`KismetSystemLibrary.Delay` 20.0)
  (`self.K2_DestroyActor`))

(event `self.Sphere.OnComponentEndOverlap`
  (params (OverlappedComponent :type "PrimitiveComponent Object Reference") (OtherActor :type "Actor Object Reference") (OtherComp :type "PrimitiveComponent Object Reference") (OtherBodyIndex :type Integer))
  (bind _returnvalue (== (`Actor.RootComponent` OtherActor) OtherComp))
  (bind _asenemy_1 (cast `/Game/Blueprints/Enemy1` OtherActor)
    (:`then`
      (if _returnvalue
        (`AIPerceptionComponent.SetSenseEnabled` (`AIController.GetAIPerceptionComponent` (`AIBlueprintHelperLibrary.GetAIController` _asenemy_1)) "/Script/AIModule.AISense_Sight" true)))
    (:`CastFailed`
      (bind _asprotagonist (cast `/Game/Blueprints/Protagonist` OtherActor))
      (if _returnvalue
        (`AIPerceptionStimuliSourceComponent.RegisterForSense` (`/Game/Blueprints/Protagonist.AIPerceptionStimuliSource` _asprotagonist) "/Script/AIModule.AISense_Sight")
        (set `/Game/Blueprints/Protagonist.Invisible` false _asprotagonist)))))

(fn `UserConstructionScript`)