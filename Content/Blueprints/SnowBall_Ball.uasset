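; Snowball projectile that freezes or roots enemies on impact.
; A hit on an Enemy1 deals damage, then can stun it with zero time dilation, disabled sight, a behavior tree blackboard flag and a snow material.
; Timers call the enemy's Cancel Stun and, if it was investigating, its controller's Endinvestigation.
; Other impacts spawn a FrostCloud and root enemies overlapping the explosion radius before the ball destroys itself.
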(event `self.ReceiveHit`
  (params (MyComp :type "PrimitiveComponent Object Reference") (Other :type "Actor Object Reference") (OtherComp :type "PrimitiveComponent Object Reference") (bSelfMoved :type Boolean) (HitLocation :type "Vector Structure") (HitNormal :type "Vector Structure") (NormalImpulse :type "Vector Structure") (Hit :type "HitResult Structure (by ref)"))
  (bind _asenemy_1 (cast `/Game/Blueprints/Enemy1` Other)
    (:`then`
      (`Enemy.takeDamage` _asenemy_1 20.0 (`self.K2_GetActorLocation` (`self.GetInstigator`)))
      (if (!= _asenemy_1 null)
        (set `Actor.CustomTimeDilation` 0.0 _asenemy_1)
        (set `/Game/Blueprints/Enemy1.Stunned` true _asenemy_1)
        (bind _asenemy_1aicontroller (cast `/Game/Blueprints/Enemy1AIController` (`Pawn.GetController` _asenemy_1)))
        (bind _returnvalue (`AIController.GetAIPerceptionComponent` _asenemy_1aicontroller))
        (`AIPerceptionComponent.SetSenseEnabled` _returnvalue "/Script/AIModule.AISense_Sight" false)
        (`AIPerceptionComponent.ForgetAll` _returnvalue)
        (bind _returnvalue_2 (`AIBlueprintHelperLibrary.GetBlackboard` _asenemy_1aicontroller))
        (`BlackboardComponent.SetValueAsBool` _returnvalue_2 "Behavior Tree Deactivated" true)
        (`KismetSystemLibrary.K2_SetTimer` _asenemy_1 "Cancel Stun" 6.5)
        (`PrimitiveComponent.SetMaterial` (`Character.Mesh` _asenemy_1) 0 "/Game/Snowball_Material.Snowball_Material")
        (if (`BlackboardComponent.GetValueAsBool` _returnvalue_2 "Investigating")
          (bind _returnvalue_3 (`KismetSystemLibrary.K2_SetTimer` _asenemy_1aicontroller "Endinvestigation" 21.5))
          (set `/Game/Blueprints/Enemy1AIController.end investigation timer` _returnvalue_3 _asenemy_1aicontroller)
          (`self.K2_DestroyActor`)
          (else
            (`self.K2_DestroyActor`)))
        (else
          (`self.K2_DestroyActor`))))
    (:`CastFailed`
      (`self.Explodeball` HitLocation))))

(fn `Ad`
  (`KismetSystemLibrary.PrintString` "Hello"))

(fn `Cancel stun`
  (bind _stun_target (`self.Stun target`))
  (set `/Game/Blueprints/Enemy1.Stunned` false _stun_target)
  (bind _asenemy_1aicontroller (cast `/Game/Blueprints/Enemy1AIController` (`Pawn.GetController` _stun_target)))
  (`Controller.Possess` _asenemy_1aicontroller _stun_target)
  (`Controller.Possess` (`Pawn.LastHitBy` _stun_target) _stun_target)
  (`KismetSystemLibrary.PrintString` (`KismetSystemLibrary.GetDisplayName` _stun_target))
  (`PrimitiveComponent.SetMaterial` (`Character.Mesh` _stun_target) 0 (`Enemy.baseenemymaterial` _stun_target)))

(fn `Explodeball`
  (params (`Hit location` :type "Vector Structure"))
  (`|SpawnActorFromClass` "/Game/FrostCloud.FrostCloud_C" (`KismetMathLibrary.Conv_VectorToTransform` `Hit location`) "Undefined" "OverrideRootScale" null null)
  (for _array_element (`PrimitiveComponent.GetOverlappingActors` (`self.Explosionradius`) "/Script/MyProject7.Enemy")
    (bind _asenemy_1 (cast `/Game/Blueprints/Enemy1` _array_element))
    (`/Game/Blueprints/Enemy1.Root` _asenemy_1))
  (`self.K2_DestroyActor`))

(fn `UserConstructionScript`)